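; BP_NaviSupervisor manages a sliding window of hints, likely audio cues, that guide the player through an ordered Hints array.
; ActiveHelpInTime starts it after a delay unless CancelHelp clears the flag first.
; Each pick advances the window, re-enabling and rebinding its hints until all are picked.
; A self-recalling delay loop, started through a DoOnce, cycles CallHint across the window while Activated.
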(event Custom|ActiveHintSupervisor
  (bind _hints (Variables|HelpsParameter|GetHints))
  (bind _returnvalue (Utilities|Array|Length _hints))
  (Utilities|FlowControl|Sequence
    (:then_0
      (if (== (Variables|Default|GetMinVisibleIndex) (Utilities|Array|Length (Variables|HelpsParameter|GetHints)))
        (Variables|Default|SetActivated false)
        (else
          (for _index (range 0 (- _returnvalue 1))
            (EventDispatchers|UnbindEventfromOnPick (Utilities|Array|Get(acopy) (Variables|HelpsParameter|GetHints) _index) (delegate Custom|OnPickReact)))
          (bind _index_2 (Utilities|FlowControl|ForLoopwithBreak (Variables|Default|GetMinVisibleIndex) (Math|Integer|Clamp(Integer) (+ (Variables|Default|GetMinVisibleIndex) (Variables|HelpsParameter|GetMaxVisibleHints)) 0 (- _returnvalue 1)))
            (:LoopBody
              (Utilities|FlowControl|Sequence
                (:then_0
                  (Default|EnableHints (Utilities|Array|Get(acopy) (Variables|HelpsParameter|GetHints) _index_2))
                  (EventDispatchers|BindEventtoOnPick (Utilities|Array|Get(acopy) (Variables|HelpsParameter|GetHints) _index_2) (delegate Custom|OnPickReact)))))
            (:Completed
              (Variables|Default|SetCurrentIteration (Math|Integer|Clamp(Integer) (Variables|Default|GetCurrentIteration) (Variables|Default|GetMinVisibleIndex) (Math|Integer|Clamp(Integer) (+ (Variables|Default|GetMinVisibleIndex) (Variables|HelpsParameter|GetMaxVisibleHints)) 0 (- _returnvalue 1)))))))))
    (:then_1
      (Utilities|FlowControl|DoOnce false
        (:Completed
          (Variables|Default|SetActivated true)
          (CallFunction|ExecuteTimer)
          (Variables|Default|SetCurrentIteration 0)
          (Variables|Default|SetMinVisibleIndex 0))))))

(event Custom|CustomEvent_0)

(event Custom|ExecuteTimer
  (bind _minvisibleindex (Variables|Default|GetMinVisibleIndex))
  (bind _maxvisiblehints (Variables|HelpsParameter|GetMaxVisibleHints))
  (bind _hints (Variables|HelpsParameter|GetHints))
  (bind _returnvalue (+ _minvisibleindex _maxvisiblehints))
  (if (Variables|Default|GetActivated)
    (Utilities|FlowControl|Delay (Variables|HelpsParameter|GetDelayBetweenCall))
    (Default|CallHint (Utilities|Array|Get(acopy) _hints (Variables|Default|GetCurrentIteration)))
    (bind _output_get (Variables|Default|SetCurrentIteration (Math|Integer|Clamp(Integer) (+ (Variables|Default|GetCurrentIteration) 1) (Variables|Default|GetMinVisibleIndex) (Math|Integer|Clamp(Integer) _returnvalue _returnvalue (- (Utilities|Array|Length _hints) 1)))))
    (if (== _output_get _returnvalue)
      (Variables|Default|SetCurrentIteration (Variables|Default|GetMinVisibleIndex)))
    (CallFunction|ExecuteTimer)))

(event Custom|OnPickReact
  (Math|Integer|IncrementInt (Variables|Default|GetMinVisibleIndex)
    (:%20%20
      (CallFunction|ActiveHintSupervisor))))

(event Custom|ActiveHelpInTime
  (params (Delay :type Float%20%28single-precision%29))
  (Variables|Default|SetActiveHints true)
  (Utilities|FlowControl|Delay Delay)
  (if (Variables|Default|GetActiveHints)
    (CallFunction|ActiveHintSupervisor)))

(event Custom|CancelHelp
  (Variables|Default|SetActiveHints false))

(event EventBeginPlay)

(event Collision|EventActorBeginOverlap
  (params (OtherActor :type Actor%20Object%20Reference)))

(event EventTick
  (params (DeltaSeconds :type Float%20%28single-precision%29)))

(fn ConstructionScript)