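; BP_Navi is a hidden audio hint pickup that becomes visible and collidable when hints are enabled, deferring parent BeginPlay until then.
; CallHint plays a randomized positional sound and enables Tick for a set duration.
; Tick samples the sound's amplitude to drive the dynamic material's Intensity, making the mesh pulse.
; Player pawn overlap calls CallOnPick, then shrinks the mesh through a recursive delay loop before hiding it and restoring its scale.
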(event OnComponentBeginOverlap(PickArea)
  (params (OverlappedComponent :type Primitive%20Component%20Object%20Reference) (OtherActor :type Actor%20Object%20Reference) (OtherComp :type Primitive%20Component%20Object%20Reference) (OtherBodyIndex :type Integer) (bFromSweep :type Boolean) (SweepResult :type Hit%20Result%20Structure%20%28by%20ref%29))
  (if (== OtherActor (Game|Player|GetPlayerPawn 0))
    (Default|CallOnPick)
    (Collision|SetCollisionEnabled (Variables|Default|GetPickArea) "NoCollision")
    (CallFunction|ExecutePick)))

(event Custom|CallHint
  (CallFunction|PlayHint)
  (Variables|Default|SetActivated true)
  (CallFunction|Timer)
  (Actor|Tick|SetActorTickEnabled true))

(event Custom|Timer
  (Utilities|FlowControl|Delay (Variables|NaviParameters|GetDuration))
  (Variables|Default|SetActivated false)
  (Rendering|Material|SetScalarParameterValue (Variables|Default|GetPulsingMat) "Intensity" 0.0 :!class /Script/Engine.MaterialInstanceDynamic)
  (Actor|Tick|SetActorTickEnabled false))

(event Custom|ExecutePick
  (bind _returnvalue (Utilities|Time|GetWorldDeltaSeconds))
  (bind _rendering (Variables|Default|GetRendering))
  (bind _returnvalue_2 (Transformation|GetWorldScale _rendering))
  (Transformation|SetWorldScale3D _rendering (Math|Vector|Lerp(Vector) _returnvalue_2 "0, 0, 0" (* _returnvalue 2.0)))
  (if (>= (Math|Vector|VectorLengthSquared _returnvalue_2) 0.0001)
    (Utilities|FlowControl|Delay _returnvalue)
    (CallFunction|ExecutePick)
    (else
      (Rendering|SetVisibility (Variables|Default|GetDefaultSceneRoot) false true)
      (Transformation|SetWorldScale3D (Variables|Default|GetRendering) (Variables|Default|GetInitialScale)))))

(event Custom|EnableHints
  (Variables|Default|SetAutoStart false)
  (|CallParentFunction)
  (Rendering|SetVisibility (Variables|Default|GetDefaultSceneRoot) true false)
  (Rendering|SetVisibility (Variables|Default|GetRendering) true false)
  (Collision|SetCollisionEnabled (Variables|Default|GetPickArea) "QueryOnly"))

(event EventBeginPlay
  (bind _pickarea (Variables|Default|GetPickArea))
  (Components|Sphere|SetSphereRadius _pickarea (Variables|NaviParameters|GetColliderRadius) true)
  (Rendering|SetVisibility (Variables|Default|GetDefaultSceneRoot) false true)
  (Collision|SetCollisionEnabled _pickarea "NoCollision")
  (Variables|Default|SetInitialScale (Transformation|GetWorldScale (Variables|Default|GetRendering))))

(event Collision|EventActorBeginOverlap
  (params (OtherActor :type Actor%20Object%20Reference)))

(event EventTick
  (params (DeltaSeconds :type Float%20%28single-precision%29))
  (if (Variables|Default|GetActivated)
    (bind _outamplitudes (Class|SoundVisualizationStatics|GetAmplitude (Variables|NaviParameters|GetSoundToEmit) 0 0.0 (Variables|NaviParameters|GetDuration) 1))
    (bind _output_get (Variables|Default|SetAmplitude _outamplitudes))
    (Rendering|Material|SetScalarParameterValue (Variables|Default|GetPulsingMat) "Intensity" (Math|Float|Lerp (Variables|Default|GetValueToLerp) (Utilities|Array|Get(acopy) _output_get) DeltaSeconds) :!class /Script/Engine.MaterialInstanceDynamic)))

(fn ConstructionScript
  (|CallParentFunction)
  (bind _returnvalue (Rendering|Material|CreateDynamicMaterialInstance (Variables|Default|GetRendering) 0 (Rendering|Material|GetMaterial (Variables|Default|GetRendering) 0) "None" :!class /Script/Engine.PrimitiveComponent))
  (bind _output_get (Variables|Default|SetPulsingMat _returnvalue))
  (Rendering|Material|SetScalarParameterValue _output_get "Intensity" 0.0 :!class /Script/Engine.MaterialInstanceDynamic))

(fn PlayHint
  (bind _volumescale (Variables|Default|GetVolumeScale))
  (Audio|PlaySoundatLocation (Variables|NaviParameters|GetSoundToEmit) (Transformation|GetWorldLocation (Variables|Default|GetDefaultSceneRoot)) "0, 0, 0" (* (Math|Random|RandomFloatinRange (Variables|Default|GetMinVolume) (Variables|Default|GetMaxVolume)) (select (Utilities|IsValid _volumescale) (Variables|/Game/1-PROJECT_LDJ/Production/Blueprints/Assets/FloatVariable.FloatVariable_C|GetValue _volumescale) 1.0)) (* (Math|Random|RandomFloatinRange (Variables|Default|GetMinPitch) (Variables|Default|GetMaxPitch)) (Variables|Default|GetPitchScale)) 0.0 (Variables|Default|GetAttenuation) (Variables|Default|GetConcurrencySettings) self))