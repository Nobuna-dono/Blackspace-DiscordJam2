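; Ambient audio actor that plays randomized bursts of a sound at its location, started automatically or when the player enters its trigger sphere.
; A random timer launches each burst of randomly spaced plays with varied volume and pitch, optionally repeating.
; BeginPlay scales the sphere from the attenuation asset's extent and falloff.
; Any end overlap sets a stop flag, checked only after a burst finishes, to prevent the next repeat.
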(event OnComponentBeginOverlap(Sphere)
  (params (OverlappedComponent :type Primitive%20Component%20Object%20Reference) (OtherActor :type Actor%20Object%20Reference) (OtherComp :type Primitive%20Component%20Object%20Reference) (OtherBodyIndex :type Integer) (bFromSweep :type Boolean) (SweepResult :type Hit%20Result%20Structure%20%28by%20ref%29))
  (if (== OtherActor (Game|Player|GetPlayerPawn 0))
    (Variables|Default|SetStopSpawner false)
    (CallFunction|ExecuteTimer)))

(event OnComponentEndOverlap(Sphere)
  (params (OverlappedComponent :type Primitive%20Component%20Object%20Reference) (OtherActor :type Actor%20Object%20Reference) (OtherComp :type Primitive%20Component%20Object%20Reference) (OtherBodyIndex :type Integer))
  (Variables|Default|SetStopSpawner true))

(event Custom|ExecuteSequence
  (Variables|SpawnParameters|SetNumberOfSpawns (Math|Random|RandomIntegerinRange (Variables|SpawnParameters|GetMinSpawns) (Variables|SpawnParameters|GetMaxSpawns)))
  (Variables|SpawnParameters|SetSpawnCount 0)
  (if (< (Variables|SpawnParameters|GetSpawnCount) (Variables|SpawnParameters|GetNumberOfSpawns)) :!label _label
    (CallFunction|PlayWordPhrase (Variables|MainParameters|GetSoundToSpawn))
    (Math|Integer|IncrementInt (Variables|SpawnParameters|GetSpawnCount)
      (:%20%20
        (Utilities|FlowControl|Delay (Math|Random|RandomFloatinRange (Variables|SpawnParameters|GetMinStepDuration) (Variables|SpawnParameters|GetMaxStepDuration)))
        (goto _label)))
    (elif (and (Variables|MainParameters|GetRepeat) (not (Variables|Default|GetStopSpawner)))
      (CallFunction|ExecuteTimer))))

(event Custom|Execute%20Timer
  (Utilities|Time|SetTimerbyEvent (delegate Custom|ExecuteSequence) (Math|Random|RandomFloatinRange (Variables|QuantityParameters|GetMinTimer) (Variables|QuantityParameters|GetMaxTimer))))

(event EventBeginPlay
  (CallFunction|InitializeTriggerSphere)
  (if (Variables|MainParameters|GetAutoStart)
    (CallFunction|ExecuteTimer)))

(fn ConstructionScript)

(fn InitializeTriggerSphere
  (bind _attenuation (Variables|MainParameters|GetAttenuation))
  (bind _attenuation_2 (Variables|/Script/Engine.SoundAttenuation|GetAttenuation _attenuation))
  (bind (_battenuate _bspatialize _battenuatewithlpf _benablelistenerfocus _benablefocusinterpolation _benableocclusion _busecomplexcollisionforocclusion _benablereverbsend _bapplynormalizationtostereosounds _benablelogfrequencyscaling _spatializationalgorithm _absorptionmethod _occlusiontracechannel _reverbsendmethod _omniradius _stereospread _lpfradiusmin _lpfradiusmax _customlowpassairabsorptioncurve _customhighpassairabsorptioncurve _lpffrequencyatmin _lpffrequencyatmax _hpffrequencyatmin _hpffrequencyatmax _focusazimuth _nonfocusazimuth _focusdistancescale _nonfocusdistancescale _focuspriorityscale _nonfocuspriorityscale _focusvolumeattenuation _nonfocusvolumeattenuation _focusattackinterpspeed _focusreleaseinterpspeed _occlusionlowpassfilterfrequency _occlusionvolumeattenuation _occlusioninterpolationtime _reverbwetlevelmin _reverbwetlevelmax _reverbdistancemin _reverbdistancemax _manualreverbsendlevel _customreverbsendcurve _pluginsettings _distancealgorithm _attenuationshape _dbattenuationatmax _attenuationshapeextents _coneoffset _falloffdistance) (Utilities|Struct|BreakSoundAttenuationSettings _attenuation_2))
  (bind _x (Math|Vector|BreakVector _attenuationshapeextents))
  (bind _returnvalue (+ _x _falloffdistance))
  (bind _returnvalue_2 (/ _returnvalue 3e+01))
  (Utilities|IsValid (Variables|MainParameters|GetAttenuation)
    (:Is%20Valid
      (Transformation|SetWorldScale3D (Variables|Default|GetSphere) (Math|Vector|MakeVector _returnvalue_2 _returnvalue_2 _returnvalue_2)))))

(fn PlayWordPhrase
  (params (InSound :type Sound%20Base%20Object%20Reference))
  (bind _volumescale (Variables|OutputParameters|GetVolumeScale))
  (Audio|PlaySoundatLocation InSound (Transformation|GetWorldLocation (Variables|Default|GetDefaultSceneRoot)) "0, 0, 0" (* (Math|Random|RandomFloatinRange (Variables|OutputParameters|GetMinVolume) (Variables|OutputParameters|GetMaxVolume)) (select (Utilities|IsValid _volumescale) (Variables|/Game/1-PROJECT_LDJ/Production/Blueprints/Assets/FloatVariable.FloatVariable_C|GetValue _volumescale) 1.0)) (* (Math|Random|RandomFloatinRange (Variables|OutputParameters|GetMinPitch) (Variables|OutputParameters|GetMaxPitch)) (Variables|OutputParameters|GetPitchScale)) 0.0 (Variables|MainParameters|GetAttenuation) (Variables|MainParameters|GetConcurrencySettings) self))