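; Base platform that can be pulled to a target position with a space-warp effect, then return to where it started.
; AttractToPosition plays a timeline that lerps the mesh's location and drives its scale and WarpFactor material parameter, alongside a sound and post-process warp.
; ResetPosition, during forward motion, freezes the platform where it is and reverses the timeline after a standstill delay.
; It becomes movable again once the reverse finishes.
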(event Custom|MovedToAttractedLoc
  (params (ToPosition :type Vector))
  (if (Variables|Default|GetCanBeMoved)
    (Audio|PlaySoundatLocation "/Game/1-PROJECT_LDJ/Production/Blueprints/Audio/SoundEffects/SpaceShift_Cue.SpaceShift_Cue" ToPosition "0, 0, 0" (Math|Random|RandomFloatinRange 0.9 1.0) (Math|Random|RandomFloatinRange 0.8 1.0) 0.0 0 0 0)
    (Variables|Default|SetCanBeMoved false)
    (Variables|Default|SetIsMoving true)
    (Variables|Default|SetArrivedAtDest false)
    (Variables|Default|SetEndPos ToPosition)
    (Variables|Default|SetStartPos (Transformation|GetWorldLocation (Variables|Default|GetStaticMesh)))
    (Default|SpaceWrap (Variables|Default|GetPostProcess))
    (bind (_direction _position _wrapfactor _scalefactor) (Timeline|WrapTimeline Play)
      (:Update
        (Transformation|SetWorldScale3D (Variables|Default|GetStaticMesh) (* (Variables|Default|GetInitialScale) (* _scalefactor (Variables|Default|GetWrapIntensity))))
        (Rendering|Material|SetScalarParameterValueonMaterials (Variables|Default|GetStaticMesh) "WarpFactor" (* (Variables|Default|GetWrapIntensity) _wrapfactor))
        (if (not (Variables|Default|GetArrivedAtDest))
          (Transformation|SetWorldLocation (Variables|Default|GetStaticMesh) (Math|Vector|Lerp(Vector) (Variables|Default|GetStartPos) (Variables|Default|GetEndPos) _position) false false)))
      (:Finished
        (switch Utilities|FlowControl|Switch|SwitchonETimelineDirection _direction
          (:Backward
            (Variables|Default|SetCanBeMoved true)
            (Variables|Default|SetIsMoving false)))))))

(event Custom|ResetPosition
  (if (Variables|Default|GetIsMoving)
    (switch Utilities|FlowControl|Switch|SwitchonETimelineDirection (stale Custom|MovedToAttractedLoc _direction)
      (:Forward
        (Variables|Default|SetIsMoving false)
        (Utilities|Time|SetTimerbyEvent (delegate Custom|StartReverseAttraction) (Variables|Default|GetStandingStillDuration))
        (Variables|Default|SetArrivedAtDest true)
        (Variables|Default|SetEndPos (Transformation|GetWorldLocation (Variables|Default|GetStaticMesh)))))))

(event Custom|StartReverseAttraction
  (Variables|Default|SetArrivedAtDest false)
  (Variables|Default|SetIsMoving true)
  (Audio|PlaySoundatLocation "/Game/1-PROJECT_LDJ/Production/Blueprints/Audio/SoundEffects/SpaceShiftReverse_Cue.SpaceShiftReverse_Cue" (Transformation|GetActorLocation) "0, 0, 0" (Math|Random|RandomFloatinRange 0.9 1.0) (Math|Random|RandomFloatinRange 0.8 1.0) 0.0 0 0 0)
  (bind (_direction _position _wrapfactor _scalefactor) (Timeline|WrapTimeline Reverse)
    (:Update
      (Transformation|SetWorldScale3D (Variables|Default|GetStaticMesh) (* (Variables|Default|GetInitialScale) (* _scalefactor (Variables|Default|GetWrapIntensity))))
      (Rendering|Material|SetScalarParameterValueonMaterials (Variables|Default|GetStaticMesh) "WarpFactor" (* (Variables|Default|GetWrapIntensity) _wrapfactor))
      (if (not (Variables|Default|GetArrivedAtDest))
        (Transformation|SetWorldLocation (Variables|Default|GetStaticMesh) (Math|Vector|Lerp(Vector) (Variables|Default|GetStartPos) (Variables|Default|GetEndPos) _position) false false)))
    (:Finished
      (switch Utilities|FlowControl|Switch|SwitchonETimelineDirection _direction
        (:Backward
          (Variables|Default|SetCanBeMoved true)
          (Variables|Default|SetIsMoving false))))))

(event EventBeginPlay
  (bind _outactors (Actor|GetAllActorsOfClass "/Game/1-PROJECT_LDJ/Production/VFX/PostProcess/BP_PostProcess.BP_PostProcess_C"))
  (Variables|Default|SetPostProcess (Utilities|Array|Get(acopy) _outactors)))

(fn ConstructionScript
  (Variables|Default|SetInitialScale (Transformation|GetWorldScale (Variables|Default|GetStaticMesh))))

(fn AttracttoPosition
  (params (ToPosition :type Vector))
  (CallFunction|MovedtoAttractedLoc ToPosition))