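; Base platform actor whose static mesh can be pulled toward a given world position, judging by its attraction functions.
; AttractToPosition triggers a timeline that lerps the mesh from its current location to the target, with a CanBeMoved flag blocking new moves until it finishes.
; ResetPosition stops the timeline and sets a timer that reverses it after StandingStillDuration, sending the mesh back toward its start.
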(event Custom|MovedToAttractedLoc
  (params (ToPosition :type Vector))
  (if (Variables|Default|GetCanBeMoved)
    (Variables|Default|SetCanBeMoved false)
    (Variables|Default|SetStartPos (Transformation|GetWorldLocation (Variables|Default|GetStaticMesh)))
    (bind _newtrack_1 (Timeline|Timeline_0 PlayFromStart)
      (:Update
        (Transformation|SetWorldLocation (Variables|Default|GetStaticMesh) (Math|Vector|Lerp(Vector) (Variables|Default|GetStartPos) ToPosition _newtrack_1) false false))
      (:Finished
        (Variables|Default|SetCanBeMoved true)))))

(event Custom|ResetPosition
  (Utilities|Time|SetTimerbyEvent (delegate Custom|StartReverseAttraction) (Variables|Default|GetStandingStillDuration))
  (bind _newtrack_1 (Timeline|Timeline_0 Stop)
    (:Update
      (Transformation|SetWorldLocation (Variables|Default|GetStaticMesh) (Math|Vector|Lerp(Vector) (Variables|Default|GetStartPos) (stale Custom|MovedToAttractedLoc ToPosition) _newtrack_1) false false))
    (:Finished
      (Variables|Default|SetCanBeMoved true))))

(event Custom|StartReverseAttraction
  (bind _newtrack_1 (Timeline|Timeline_0 Reverse)
    (:Update
      (Transformation|SetWorldLocation (Variables|Default|GetStaticMesh) (Math|Vector|Lerp(Vector) (Variables|Default|GetStartPos) (stale Custom|MovedToAttractedLoc ToPosition) _newtrack_1) false false))
    (:Finished
      (Variables|Default|SetCanBeMoved true))))

(event EventBeginPlay)

(event Collision|EventActorBeginOverlap
  (params (OtherActor :type Actor%20Object%20Reference)))

(fn ConstructionScript)

(fn AttracttoPosition
  (params (ToPosition :type Vector))
  (CallFunction|MovedtoAttractedLoc ToPosition))