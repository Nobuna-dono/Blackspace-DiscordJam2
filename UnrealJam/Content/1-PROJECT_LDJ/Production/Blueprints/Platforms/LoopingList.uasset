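; LoopingList is a cursor over TransformArray that steps to the next or previous transform, apparently for platform paths.
; GetNext and GetPrevious use the Reverse flag to choose between wrap-around looping and ping-pong traversal, which flips Forward at the ends.
; Each helper updates or checks CurrentIndex and returns the transform there.
; The upper-bound checks compare CurrentIndex - 1 to the array length, letting forward stepping overrun the last element.
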(event EventBeginPlay)

(event EventTick
  (params (DeltaSeconds :type Float%20%28single-precision%29)))

(fn GetNext
  (if (Variables|Default|Getreverse)
    (CallFunction|GetReverseNext)
    (else
      (bind _nexttransform (CallFunction|GetLoopingNext))))
  (return _nexttransform))

(fn GetPrevious
  (if (Variables|Default|Getreverse)
    (CallFunction|GetReversePrevious)
    (else
      (bind _previoustransform (CallFunction|GetLoopingPrevious))))
  (return _previoustransform))

(fn GetLoopingNext
  (if (>= (- (Variables|Default|GetcurrentIndex) 1) (Utilities|Array|Length (Variables|Default|GetTransformArray)))
    (Variables|Default|SetcurrentIndex 0)
    (else
      (Math|Integer|IncrementInt (Variables|Default|GetcurrentIndex)
        (:%20%20
          _))))
  (return (Utilities|Array|Get(acopy) (Variables|Default|GetTransformArray) (Variables|Default|GetcurrentIndex))))

(fn GetLoopingPrevious
  (if (<= (Variables|Default|GetcurrentIndex) 0)
    (Variables|Default|SetcurrentIndex (- (Utilities|Array|Length (Variables|Default|GetTransformArray)) 1))
    (else
      (Math|Integer|DecrementInt (Variables|Default|GetcurrentIndex)
        (:%20%20
          _))))
  (return (Utilities|Array|Get(acopy) (Variables|Default|GetTransformArray) (Variables|Default|GetcurrentIndex))))

(fn GetReverseNext
  (bind _currentindex (Variables|Default|GetcurrentIndex))
  (if (Variables|Default|Getforward)
    (if (>= (- (Variables|Default|GetcurrentIndex) 1) (Utilities|Array|Length (Variables|Default|GetTransformArray)))
      (Variables|Default|Setforward (not (Variables|Default|Getforward)))
      (Math|Integer|DecrementInt _currentindex
        (:%20%20
          _))
      (else
        (Math|Integer|IncrementInt _currentindex
          (:%20%20
            _))))
    (elif (<= (Variables|Default|GetcurrentIndex) 0)
      (Variables|Default|Setforward (not (Variables|Default|Getforward)))
      (Math|Integer|IncrementInt _currentindex
        (:%20%20
          _))
      (else
        (Math|Integer|DecrementInt _currentindex
          (:%20%20
            _)))))
  (return (Utilities|Array|Get(acopy) (Variables|Default|GetTransformArray) (Variables|Default|GetcurrentIndex))))

(fn GetReversePrevious
  (bind _currentindex (Variables|Default|GetcurrentIndex))
  (if (Variables|Default|Getforward)
    (if (<= (Variables|Default|GetcurrentIndex) 0)
      (Variables|Default|Setforward (not (Variables|Default|Getforward)))
      (Math|Integer|IncrementInt (stale _result)
        (:%20%20
          _))
      (else
        (bind _result (Math|Integer|DecrementInt _currentindex)
          (:%20%20
            _))))
    (elif (>= (- (Variables|Default|GetcurrentIndex) 1) (Utilities|Array|Length (Variables|Default|GetTransformArray)))
      (Variables|Default|Setforward (not (Variables|Default|Getforward)))
      (Math|Integer|DecrementInt (stale _result_2)
        (:%20%20
          _))
      (else
        (bind _result_2 (Math|Integer|IncrementInt _currentindex)
          (:%20%20
            _)))))
  (return (Utilities|Array|Get(acopy) (Variables|Default|GetTransformArray) (Variables|Default|GetcurrentIndex))))