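; Moving platform that travels between transforms supplied by a LoopingList, pausing for a waiting time at each stop.
; Tick alternates between a cooldown timer, which fetches the next transform when it expires, and interpolated travel that ends within a tolerance, effectively ignoring scale.
; Location eases via VInterpTo, while RInterpTo receives the target rotation as Current and the actor's as Target, reversing the usual order.
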(event EventBeginPlay)

(event Collision|EventActorBeginOverlap
  (params (OtherActor :type Actor%20Object%20Reference)))

(event EventTick
  (params (DeltaSeconds :type Float%20%28single-precision%29))
  (if (Variables|Default|Gettravelling)
    (CallFunction|PlatformTraveling DeltaSeconds)
    (else
      (CallFunction|ComputeCooldownTravel DeltaSeconds))))

(fn ConstructionScript)

(fn ComputeCooldownTravel
  (params (deltaTime :type Float%20%28single-precision%29))
  (bind _loopinglist (Variables|Default|GetLoopingList))
  (bind _output_get (Variables|Default|SetcurrentTime (+ deltaTime (Variables|Default|GetcurrentTime))))
  (if (>= _output_get (Variables|Default|GetwaitingTime))
    (Variables|Default|Settravelling true)
    (Variables|Default|SetcurrentTime 0.0)
    (Utilities|IsValid _loopinglist
      (:Is%20Valid
        (bind _nexttransform (Default|GetNext _loopinglist))
        (Variables|Default|SetnextTransform _nexttransform)))))

(fn PlatformTraveling
  (params (deltaTime :type Float%20%28single-precision%29))
  (bind _self self)
  (bind _nexttransform (Variables|Default|GetnextTransform))
  (bind _tolerance (Variables|Default|Gettolerance))
  (bind (_location _rotation) (Math|Transform|BreakTransform _nexttransform))
  (LocalVariables|SetpDeltaTime deltaTime)
  (Transformation|SetActorLocationAndRotation (Math|Interpolation|VInterpTo (Transformation|GetActorLocation self) _location (LocalVariables|GetpDeltaTime) (Variables|Default|GettravelSpeed)) (Math|Interpolation|RInterpTo _rotation (Transformation|GetActorRotation _self) (LocalVariables|GetpDeltaTime) (Variables|Default|GettravelSpeed)))
  (if (Class|KismetMathLibrary|NearlyEqualTransformTransform (Variables|Default|GetnextTransform) (Transformation|GetActorTransform _self) _tolerance _tolerance 2.00376414667119e+18)
    (Variables|Default|Settravelling false)))