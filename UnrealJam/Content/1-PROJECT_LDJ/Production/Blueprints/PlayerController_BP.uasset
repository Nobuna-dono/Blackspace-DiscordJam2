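; Player controller that routes player input to the controlled pawn.
; Look and turn axes add pitch and yaw input to the pawn.
; Space stretch press and release start and stop SpaceStretch on PlayerPawn_BP, and the teleport button calls its TPToAimedLocation, each through a cast.
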(event EventBeginPlay)

(event EventTick
  (params (DeltaSeconds :type Float%20%28single-precision%29)))

(event Input|ActionEvents|InputActionSpaceStretch
  (params (Key :type Key%20Structure))
  (bind _returnvalue (Pawn|GetControlledPawn))
  (:Pressed
    (bind _asplayer_pawn_bp (Utilities|Casting|CastToPlayerPawn_BP _returnvalue))
    (Default|SpaceStretch _asplayer_pawn_bp))
  (:Released
    (bind _asplayer_pawn_bp_2 (Utilities|Casting|CastToPlayerPawn_BP _returnvalue))
    (Default|StopSpaceStretch _asplayer_pawn_bp_2)))

(event Input|ActionEvents|InputActionTpButton
  (params (Key :type Key%20Structure))
  (:Pressed
    (bind _asplayer_pawn_bp (Utilities|Casting|CastToPlayerPawn_BP (Pawn|GetControlledPawn)))
    (Default|TPtoAimedLocation _asplayer_pawn_bp)))

(event Input|AxisEvents|InputAxisLookUp
  (params (AxisValue :type Float%20%28single-precision%29))
  (Pawn|Input|AddControllerPitchInput (Pawn|GetControlledPawn) AxisValue))

(event Input|AxisEvents|InputAxisTurn
  (params (AxisValue :type Float%20%28single-precision%29))
  (Pawn|Input|AddControllerYawInput (Pawn|GetControlledPawn) AxisValue))

(fn ConstructionScript)