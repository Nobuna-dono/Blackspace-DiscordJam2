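; Base platform that can be attracted to a target position, warping as it travels, then return to where it started.
; AttractToPosition plays one timeline that lerps the mesh location while driving its scale and a WarpFactor material parameter.
; ResetPosition freezes movement at the current spot, then after StandingStillDuration reverses the same timeline.
; CanBeMoved blocks new attraction until the reverse playback finishes.
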(event Custom|MovedToAttractedLoc
  (params (ToPosition :type Vector))
  (if (Variables|Default|GetCanBeMoved)
    (Variables|Default|SetCanBeMoved false)
    (Variables|Default|SetArrivedAtDest false)
    (Variables|Default|SetEndPos ToPosition)
    (Variables|Default|SetStartPos (Transformation|GetWorldLocation (Variables|Default|GetStaticMesh)))
    (bind (_direction _position _wrapfactor _scalefactor) (Timeline|WrapTimeline Play)
      (:Update
        (Transformation|SetWorldScale3D (Variables|Default|GetStaticMesh) (* (Variables|Default|GetInitialScale) (* _scalefactor (Variables|Default|GetWrapSpeed))))
        (Rendering|Material|SetScalarParameterValueonMaterials (Variables|Default|GetStaticMesh) "WarpFactor" (* (Variables|Default|GetWrapSpeed) _wrapfactor))
        (if (not (Variables|Default|GetArrivedAtDest))
          (Transformation|SetWorldLocation (Variables|Default|GetStaticMesh) (Math|Vector|Lerp(Vector) (Variables|Default|GetStartPos) (Variables|Default|GetEndPos) (* _position (Variables|Default|GetMoveSpeed))) false false)))
      (:Finished
        (switch Utilities|FlowControl|Switch|SwitchonETimelineDirection _direction
          (:Backward
            (Variables|Default|SetCanBeMoved true)))))))

(event Custom|ResetPosition
  (Utilities|Time|SetTimerbyEvent (delegate Custom|StartReverseAttraction) (Variables|Default|GetStandingStillDuration))
  (Variables|Default|SetArrivedAtDest true)
  (Variables|Default|SetEndPos (Transformation|GetWorldLocation (Variables|Default|GetStaticMesh))))

(event Custom|StartReverseAttraction
  (Variables|Default|SetArrivedAtDest false)
  (bind (_direction _position _wrapfactor _scalefactor) (Timeline|WrapTimeline Reverse)
    (:Update
      (Transformation|SetWorldScale3D (Variables|Default|GetStaticMesh) (* (Variables|Default|GetInitialScale) (* _scalefactor (Variables|Default|GetWrapSpeed))))
      (Rendering|Material|SetScalarParameterValueonMaterials (Variables|Default|GetStaticMesh) "WarpFactor" (* (Variables|Default|GetWrapSpeed) _wrapfactor))
      (if (not (Variables|Default|GetArrivedAtDest))
        (Transformation|SetWorldLocation (Variables|Default|GetStaticMesh) (Math|Vector|Lerp(Vector) (Variables|Default|GetStartPos) (Variables|Default|GetEndPos) (* _position (Variables|Default|GetMoveSpeed))) false false)))
    (:Finished
      (switch Utilities|FlowControl|Switch|SwitchonETimelineDirection _direction
        (:Backward
          (Variables|Default|SetCanBeMoved true))))))

(event EventBeginPlay)

(event Collision|EventActorBeginOverlap
  (params (OtherActor :type Actor%20Object%20Reference)))

(fn ConstructionScript
  (Variables|Default|SetInitialScale (Transformation|GetWorldScale (Variables|Default|GetStaticMesh))))

(fn AttracttoPosition
  (params (ToPosition :type Vector))
  (CallFunction|MovedtoAttractedLoc ToPosition))