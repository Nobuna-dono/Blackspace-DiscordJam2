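; Player pawn that teleports between faces of platform actors and can pull an aimed platform toward itself (SpaceStretch).
; Teleport traces from the head, matches the hit normal to a Face_BP, and only if activated attaches to it and fires the post-process effect.
; Tick applies control yaw, negated off platform tops, sways the spring arm with yaw change and places an aim sphere at the trace hit.
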(event EventBeginPlay
  (bind _outactors (Actor|GetAllActorsOfClass "/Game/1-PROJECT_LDJ/Production/VFX/PostProcess/BP_PostProcess.BP_PostProcess_C"))
  (Variables|Default|SetPostProcess (Utilities|Array|Get(acopy) _outactors)))

(event Collision|EventActorBeginOverlap
  (params (OtherActor :type Actor%20Object%20Reference)))

(event EventTick
  (params (DeltaSeconds :type Float%20%28single-precision%29))
  (bind _returnvalue (Pawn|GetControlRotation :!class /Script/Engine.Pawn))
  (bind _onplatformtop (Variables|Default|GetOnPlatformTop))
  (bind _headrot (Variables|Default|GetHeadRot))
  (bind _returnvalue_2 (Transformation|GetWorldLocation _headrot))
  (bind _returnvalue_3 (Class|KismetMathLibrary|NegateRotator _returnvalue))
  (bind _returnvalue_4 (select _onplatformtop _returnvalue _returnvalue_3))
  (bind _yaw (Math|Rotator|BreakRotator _returnvalue_4))
  (Transformation|SetActorRelativeRotation (Math|Rotator|MakeRotator 0.0 0.0 _yaw))
  (CallFunction|SetSpringOffset DeltaSeconds (- (Variables|Default|GetYawBuff) (Math|Float|Lerp (Variables|Default|GetYawBuff) _yaw DeltaSeconds)))
  (Variables|Default|SetYawBuff _yaw)
  (bind _outhit (Collision|LineTraceByChannel _returnvalue_2 (+ _returnvalue_2 (* (Math|Vector|GetForwardVector (Variables|Default|GetCamera)) (Variables|Default|GetSpaceStretchMaxDistance))) "TraceTypeQuery1" false 0 "None"))
  (Transformation|SetWorldLocation (Variables|Default|GetSphere) (.Location (Collision|BreakHitResult _outhit)) false true))

(fn ConstructionScript)

(fn SpaceStretch
  (bind _camera (Variables|Default|GetCamera))
  (bind _returnvalue (Transformation|GetWorldLocation _camera))
  (bind (_outhit _returnvalue_2) (Collision|LineTraceByChannel _returnvalue (+ _returnvalue (* (Math|Vector|GetForwardVector _camera) (Variables|Default|GetSpaceStretchMaxDistance))) "TraceTypeQuery1" false 0 "Persistent"))
  (if _returnvalue_2
    (bind _asbase_platform_bp (Utilities|Casting|CastToBasePlatform_BP (.HitActor (Collision|BreakHitResult _outhit))))
    (if (!= _asbase_platform_bp (Variables|Default|GetCurrentPlatform))
      (bind _output_get (Variables|Default|SetTargetPlatform _asbase_platform_bp))
      (Default|AttracttoPosition _output_get (+ (Transformation|GetActorLocation) (* (Math|Vector|GetForwardVector (Variables|Default|GetCapsuleComponent)) 1e+02))))))

(fn StopSpaceStretch
  (bind _targetplatform (Variables|Default|GetTargetPlatform))
  (Utilities|IsValid _targetplatform
    (:Is%20Valid
      (Default|ResetPosition _targetplatform))))

(fn TPtoAimedLocation
  (bind _headrot (Variables|Default|GetHeadRot))
  (bind _returnvalue (Transformation|GetWorldLocation _headrot))
  (Transformation|SetWorldLocation (Variables|Default|GetCube) _returnvalue false true)
  (bind (_outhit _returnvalue_2) (Collision|LineTraceByChannel _returnvalue (+ _returnvalue (* (Math|Vector|GetForwardVector (Variables|Default|GetCamera)) (Variables|Default|GetMaximumTPDistance))) "TraceTypeQuery1" false (Utilities|Array|MakeArray (Variables|Default|GetCurrentPlatform)) "Persistent" true "(R=1.000000,G=0.000000,B=0.000000,A=1.000000)" "(R=0.000000,G=1.000000,B=0.000000,A=1.000000)" 1.0))
  (if _returnvalue_2
    (bind _asbase_platform_bp (Utilities|Casting|CastToBasePlatform_BP (.HitActor (Collision|BreakHitResult _outhit))))
    (bind _array_element (Utilities|Array|ForEachLoopwithBreak (Actor|GetComponentsByClass _asbase_platform_bp "/Game/1-PROJECT_LDJ/Production/Blueprints/Platforms/Face_BP.Face_BP_C") :!label _label)
      (:LoopBody
        (if (Math|Vector|Equal(Vector) (Math|Vector|GetUpVector _array_element) (.Normal (Collision|BreakHitResult _outhit)) 0.0001)
          (goto _label Break)))
      (:Completed
        (bind _asface_bp (Utilities|Casting|CastToFace_BP _array_element))
        (if (Variables|/Game/1-PROJECT_LDJ/Production/Blueprints/Platforms/Face_BP.Face_BP_C|GetActivated _asface_bp)
          (Variables|Default|SetOnPlatformTop (Class|KismetMathLibrary|EqualExactlyVectorVector (Transformation|GetActorUpVector (.HitActor (Collision|BreakHitResult _outhit))) (.Normal (Collision|BreakHitResult _outhit))))
          (Variables|Default|SetCurrentPlatform _asbase_platform_bp)
          (Transformation|Teleport (.Location (Collision|BreakHitResult _outhit)) (Transformation|GetWorldRotation (.HitComponent (Collision|BreakHitResult _outhit))))
          (Transformation|AttachComponentToComponent _array_element "None" "KeepWorld" "KeepWorld" "KeepWorld" false)
          (Default|TeleportEffect (Variables|Default|GetPostProcess)))))))

(fn IstheSideActivated)

(fn SetSpringOffset
  (params (Alpha :type Float%20%28single-precision%29) (NewParam :type Float%20%28single-precision%29))
  (bind _springarm (Variables|Default|GetSpringArm))
  (Variables|/Script/Engine.SpringArmComponent|SetSocketOffset _springarm (Math|Vector|Lerp(Vector) (Variables|/Script/Engine.SpringArmComponent|GetSocketOffset _springarm) (Math|Vector|MakeVector 0.0 (* NewParam (Variables|Default|GetMaxSpringOffset)) 0.0) Alpha)))