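; BP_Skybox is a skybox VFX Blueprint that continuously spins three nested torus components: inner, middle and outer.
; On Tick, each torus adds a world rotation from its own speed variable, scaled by delta seconds to stay frame-rate independent.
; The construction script is empty, so all of the behavior lives in the event graph.
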(event EventTick
  (params (DeltaSeconds :type Float%20%28single-precision%29))
  (Transformation|AddWorldRotation (Variables|Default|GetInnerTorus) (* (Variables|Default|GetInnerSpeed) DeltaSeconds) false false)
  (Transformation|AddWorldRotation (Variables|Default|GetMiddleTorus) (* (Variables|Default|GetMiddleSpeed) DeltaSeconds) false false)
  (Transformation|AddWorldRotation (Variables|Default|GetOuterTorus) (* (Variables|Default|GetOuterSpeed) DeltaSeconds) false false))

(fn ConstructionScript)