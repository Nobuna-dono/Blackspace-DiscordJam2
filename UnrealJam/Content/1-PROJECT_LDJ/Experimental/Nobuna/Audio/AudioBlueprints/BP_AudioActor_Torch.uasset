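; Torch audio actor that turns a wavetable into randomly varying sound with a granular synth.
; A looping random timer scrubs the playhead to random intensity-scaled positions, with grain envelope and duration derived from the maximum timer interval.
; Unless AutoStart is set, a sphere scaled from attenuation distance plus buffer starts and stops playback, including an initial camera distance check.
; Functions can swap the synth for an attached substitute wave and back.
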(event OnComponentBeginOverlap(Sphere)
  (params (OverlappedComponent :type Primitive%20Component%20Object%20Reference) (OtherActor :type Actor%20Object%20Reference) (OtherComp :type Primitive%20Component%20Object%20Reference) (OtherBodyIndex :type Integer) (bFromSweep :type Boolean) (SweepResult :type Hit%20Result%20Structure%20%28by%20ref%29))
  ;[1 1 1] If Not Auto Start, use Collision Sphere to Turn On and Off
  (if (not (Variables|AltWavePlayer|GetbPlayAltWave))
    (if (not (Variables|MainParameters|GetbAutoStart))
      (CallFunction|ExecutePlay)
      ;;[1 1 1] Debug Comment
      (if (Variables|MainParameters|GetbDebug)
        (Development|PrintString (Utilities|String|Append (Utilities|GetDisplayName self) " has Activated") true true "(R=0.064768,G=1.000000,B=0.000000,A=1.000000)")))))

(event OnComponentEndOverlap(Sphere)
  (params (OverlappedComponent :type Primitive%20Component%20Object%20Reference) (OtherActor :type Actor%20Object%20Reference) (OtherComp :type Primitive%20Component%20Object%20Reference) (OtherBodyIndex :type Integer))
  ;[1 1 1] If Not Auto Start, use Collision Sphere to Turn On and Off
  (if (not (Variables|AltWavePlayer|GetbPlayAltWave))
    (if (not (Variables|MainParameters|GetbAutoStart))
      (CallFunction|ExecuteStop)
      ;;[1 1 1] Debug Comment
      (if (Variables|MainParameters|GetbDebug)
        (Development|PrintString (Utilities|String|Append (Utilities|GetDisplayName self) " has Deactivated") true true "(R=1.000000,G=0.014042,B=0.000000,A=1.000000)")))))

(event Custom|ExecutePlay
  ;[1 1 1] Start Grain Synth
  (if (not (Variables|AltWavePlayer|GetbPlayAltWave))
    (Variables|Default|SetbContinueLoop true)
    (CallFunction|InitializeGranularSynth (Variables|Default|GetGranularSynth))
    (CameraShake|Start (Variables|Default|GetGranularSynth))
    (CallFunction|Noteon (Variables|Default|GetGranularSynth) 6e+01 128 -1.0)
    ;;[1 1 1] Begin Timer Loop
    (CallFunction|ExecuteTimerLoop)))

(event Custom|ExecuteGrainPlayheadMovement
  (bind _intensityscale (Variables|IntensityParameters|GetIntensityScale))
  (bind _minintensity (Variables|IntensityParameters|GetMinIntensity))
  (bind _maxintensity (Variables|IntensityParameters|GetMaxIntensity))
  (bind _wavetable (Variables|MainParameters|GetWaveTable))
  (bind _returnvalue (Math|Random|RandomFloatinRange _minintensity _maxintensity))
  (bind _duration (Variables|/Script/Engine.SoundBase|GetDuration _wavetable))
  (bind _returnvalue_2 (* _returnvalue _intensityscale))
  (bind _returnvalue_3 (Math|Float|MapRangeClamped _returnvalue_2 0.0 1.0 0.0 _duration))
  ;[1 1 1] Event Timer Loop Section
  (if (not (Variables|AltWavePlayer|GetbPlayAltWave))
    ;;[1 1 1] Move Playhead to New Location
    (CallFunction|SetPlayheadTime (Variables|Default|GetGranularSynth) _returnvalue_3 (* (Utilities|Time|GetWorldDeltaSeconds) (Variables|TimingParameters|GetInterpolationScale)))
    ;;[1 1 1] Loopback Event Timer Reset
    (Utilities|FlowControl|Sequence
      (:then_0
        (if (Variables|Default|GetbContinueLoop)
          (CallFunction|ExecuteTimerLoop)))
      (:then_1
        ;;[1 1 1] Print if Debug On
        (if (Variables|MainParameters|GetbDebug)
          (Development|PrintString (Utilities|String|ToString(Float) _returnvalue_3) true true "(R=0.000000,G=0.660000,B=1.000000,A=1.000000)" 0.4))))))

(event Custom|ExecuteStop
  ;[1 1 1] Stop Grain Synth
  (Variables|Default|SetbContinueLoop false)
  (CallFunction|NoteOff (Variables|Default|GetGranularSynth) 6e+01 true)
  (Audio|Components|Audio|Stop (Variables|Default|GetGranularSynth)))

(event Custom|ExecuteTimerLoop
  ;[1 1 1] Event Timer Loop Section
  ;;[1 1 1] Randomly Set Event Timer
  (if (not (Variables|AltWavePlayer|GetbPlayAltWave))
    (Utilities|Time|SetTimerbyEvent (delegate Custom|ExecuteGrainPlayheadMovement) (Math|Random|RandomFloatinRange (Variables|TimingParameters|GetMinDeltaTime) (Variables|TimingParameters|GetMaxDeltaTime)))))

(event EventBeginPlay
  (bind _granularsynth (Variables|Default|GetGranularSynth))
  ;[1 1 1] Initialize Grain Synth Settings
  (Variables|/Script/AudioMixer.SynthComponent|SetAttenuationSettings _granularsynth (Variables|MainParameters|GetAttenuationSettingsIn))
  (Variables|/Script/AudioMixer.SynthComponent|SetConcurrencySet _granularsynth (Utilities|Set|MakeSet (Variables|MainParameters|GetConcurrencySettingsIn)))
  (bind _bplayerinbounds (CallFunction|InitializeTriggerSphere))
  ;;[1 1 1] If AutoStart True or Player in Bounds, Run Execute Play
  (if (or _bplayerinbounds (Variables|MainParameters|GetbAutoStart))
    (CallFunction|ExecutePlay)))

(fn ConstructionScript)

(fn InitializeGranularSynth
  (params (GranularSynthComponent :type %20Object%20Reference%20%28by%20ref%29))
  (bind _maxdeltatime (Variables|TimingParameters|GetMaxDeltaTime))
  (bind _returnvalue (* _maxdeltatime 1e+03))
  (bind _returnvalue_2 (/ _returnvalue 2.0))
  (CallFunction|SetAttackTime GranularSynthComponent _returnvalue_2)
  (CallFunction|SetDecayTime GranularSynthComponent _returnvalue_2)
  (CallFunction|SetGrainDuration GranularSynthComponent _returnvalue (Math|Vector2D|MakeVector2D _returnvalue_2 _returnvalue_2))
  (CallFunction|SetGrainEnvelopeType GranularSynthComponent 0)
  (CallFunction|SetGrainPan GranularSynthComponent 0.0)
  (CallFunction|SetGrainPitch GranularSynthComponent (Variables|MainParameters|GetPitchScale) "(X=0.125000,Y=2.000000)")
  (CallFunction|SetGrainProbability GranularSynthComponent 1.0)
  (CallFunction|SetGrainVolume GranularSynthComponent (Variables|MainParameters|GetVolumeScale) "(X=0.250000,Y=1.250000)")
  (CallFunction|SetGrainsPerSecond GranularSynthComponent 4.0)
  (CallFunction|SetPlaybackSpeed GranularSynthComponent 0.0)
  (CallFunction|SetPlayheadTime GranularSynthComponent 0.0 0.0 0)
  (CallFunction|SetReleaseTimeMsec GranularSynthComponent 1e+02)
  (CallFunction|SetScrubMode GranularSynthComponent true)
  (CallFunction|SetSustainGain GranularSynthComponent 1.0)
  (CallFunction|SetSoundWave GranularSynthComponent (Variables|MainParameters|GetWaveTable)))

(fn InitializeTriggerSphere
  (bind _triggerbufferdistance (Variables|Default|GetTriggerBufferDistance))
  (bind _attenuationsettingsin (Variables|MainParameters|GetAttenuationSettingsIn))
  (bind _attenuation (Variables|/Script/Engine.SoundAttenuation|GetAttenuation _attenuationsettingsin))
  (bind _lpfradiusmax (Utilities|Struct|BreakSoundAttenuationSettings _attenuation))
  (bind _returnvalue (+ _lpfradiusmax _triggerbufferdistance))
  (bind _returnvalue_2 (/ _returnvalue 3e+01))
  ;[1 1 1] Get Max Attenuation Distance, Add Trigger Distance Buffer Amount, Divide by Radius of default Collision Sphere, get Scale Amount for scaling Collision Sphere.
  (Utilities|IsValid _attenuationsettingsin
    (:Is%20Valid
      (Transformation|SetWorldScale3D (Variables|Default|GetSphere) (Math|Vector|MakeVector _returnvalue_2 _returnvalue_2 _returnvalue_2))
      (return (>= _returnvalue (Math|Vector|VectorLength (- (Transformation|GetWorldLocation (Variables|/Script/Engine.PlayerCameraManager|GetTransformComponent (Game|GetPlayerCameraManager 0))) (Transformation|GetWorldLocation (Variables|Default|GetDefaultSceneRoot self)))))))))

(fn EnableAltWavePlayback
  (bind _substitutesoundwave (Variables|AltWavePlayer|GetSubstituteSoundWave))
  (if (and (not (Variables|AltWavePlayer|GetbPlayAltWave)) (Utilities|IsValid _substitutesoundwave))
    (Variables|AltWavePlayer|SetbPlayAltWave true)
    (CallFunction|ExecuteStop)
    (Components|Activation|Deactivate (Variables|Default|GetGranularSynth))
    (bind _returnvalue (Audio|SpawnSoundAttached (Variables|AltWavePlayer|GetSubstituteSoundWave) (Variables|Default|GetDefaultSceneRoot) "None" "0, 0, 0" "0, 0, 0" "KeepRelativeOffset" false 1.0 1.0 (* (Math|Random|RandomFloatinRange 0.0 1.0) (Variables|/Script/Engine.SoundBase|GetDuration _substitutesoundwave)) (Variables|AltWavePlayer|GetAltWaveAttenuationSettings) (Variables|MainParameters|GetConcurrencySettingsIn)))
    (Variables|Default|SetAltWavePlayer _returnvalue)
    (else
      (LocalVariables|SetbSuccessful false)))
  (return (LocalVariables|GetbSuccessful)))

(fn DisableAltWavePlayback
  (bind _altwaveplayer (Variables|Default|GetAltWavePlayer))
  (Variables|AltWavePlayer|SetbPlayAltWave false)
  (CallFunction|ExecutePlay)
  (Utilities|IsValid _altwaveplayer
    (:Is%20Valid
      (Audio|Components|Audio|Stop _altwaveplayer))))