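; Ambient audio actor that plays a sound in phrases of randomized count, spacing, volume and pitch, optionally repeating after random delays.
; Each phrase shares one location offset, though CalculateRandomLocation's random-vector math is unconnected.
; It starts on BeginPlay with AutoStart or on sphere overlap; player exit stops repeats.
; The trigger sphere scales from attenuation extent plus falloff, and EndOfPhraseAction is a stub hook.
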(event OnComponentBeginOverlap(Sphere)
  (params (OverlappedComponent :type Primitive%20Component%20Object%20Reference) (OtherActor :type Actor%20Object%20Reference) (OtherComp :type Primitive%20Component%20Object%20Reference) (OtherBodyIndex :type Integer) (bFromSweep :type Boolean) (SweepResult :type Hit%20Result%20Structure%20%28by%20ref%29))
  ;[1 1 1] if Not Auto Start, use Collision Sphere to Turn On and Off
  (if (or (== OtherActor (Game|GetPlayerCharacter 0)) (Variables|MainParameters|GetbAutoStart))
    (Variables|Default|SetbContinueSpawner true)
    (CallFunction|ExecuteTimer)))

(event OnComponentEndOverlap(Sphere)
  (params (OverlappedComponent :type Primitive%20Component%20Object%20Reference) (OtherActor :type Actor%20Object%20Reference) (OtherComp :type Primitive%20Component%20Object%20Reference) (OtherBodyIndex :type Integer))
  ;[1 1 1] if Not Auto Start, use Collision Sphere to Turn On and Off
  (if (== OtherActor (Game|GetPlayerCharacter 0))
    (Variables|Default|SetbContinueSpawner false)))

(event Custom|ExecuteSequence
  ;[1 1 1] Initialize Sequence Variables
  (Variables|QuantityParameters|SetNumberOfSpawns (Math|Random|RandomIntegerinRange (Variables|QuantityParameters|GetMinSpawns) (Variables|QuantityParameters|GetMaxSpawns)))
  (Variables|Default|SetSpawnCounter 0)
  ;[1 1 1] Exit Loop If We've Exceeded the Number of Spawns We Want
  (Variables|Default|SetPhraseLocation (Utilities|CalculateRandomLocation (Variables|SpatialParameters|GetbIncludeHeight) (Variables|SpatialParameters|GetSpawnRadius)))
  (if (< (Variables|Default|GetSpawnCounter) (Variables|QuantityParameters|GetNumberOfSpawns)) :!label _label
    ;[1 1 1] Play Word at Phrase Location
    (CallFunction|PlayWordatPhraseLocation (Variables|MainParameters|GetSoundToSpawn))
    ;[1 1 1] Iterate Spawn Counter
    (Math|Integer|IncrementInt (Variables|Default|GetSpawnCounter)
      (:%20%20
        ;[1 1 1] Delay Next Sequence Step
        (Utilities|FlowControl|Delay (Math|Random|RandomFloatinRange (Variables|TimeParameters|GetMinStepDuration) (Variables|TimeParameters|GetMaxStepDuration)))
        (goto _label)))
    (else
      ;[1 1 1] Do Any End Of Phrase Actions
      (CallFunction|EndOfPhraseAction)
      ;[1 1 1] If Repeat True, Start Another Timer
      (if (and (Variables|MainParameters|GetbRepeat) (Variables|Default|GetbContinueSpawner))
        (CallFunction|ExecuteTimer)))))

(event Custom|ExecuteTimer
  ;[1 1 1] Start an Event Timer
  (Utilities|Time|SetTimerbyEvent (delegate Custom|ExecuteSequence) (Math|Random|RandomFloatinRange (Variables|TimeParameters|GetMinTimer) (Variables|TimeParameters|GetMaxTimer))))

(event EventBeginPlay
  ;[1 1 1] Execute Timer if Auto Start True
  (CallFunction|InitializeTriggerSphere)
  (if (Variables|MainParameters|GetbAutoStart)
    (Variables|Default|SetbContinueSpawner true)
    (if (Variables|TimeParameters|GetbDelayFirstTime)
      (CallFunction|ExecuteTimer)
      (else
        (CallFunction|ExecuteSequence)))))

(fn ConstructionScript)

(fn InitializeTriggerSphere
  (bind _attenuationsettings (Variables|MainParameters|GetAttenuationSettings))
  (bind _attenuation (Variables|/Script/Engine.SoundAttenuation|GetAttenuation _attenuationsettings))
  (bind (_battenuate _bspatialize _battenuatewithlpf _benablelistenerfocus _benablefocusinterpolation _benableocclusion _busecomplexcollisionforocclusion _benablereverbsend _bapplynormalizationtostereosounds _benablelogfrequencyscaling _spatializationalgorithm _absorptionmethod _occlusiontracechannel _reverbsendmethod _omniradius _stereospread _lpfradiusmin _lpfradiusmax _customlowpassairabsorptioncurve _customhighpassairabsorptioncurve _lpffrequencyatmin _lpffrequencyatmax _hpffrequencyatmin _hpffrequencyatmax _focusazimuth _nonfocusazimuth _focusdistancescale _nonfocusdistancescale _focuspriorityscale _nonfocuspriorityscale _focusvolumeattenuation _nonfocusvolumeattenuation _focusattackinterpspeed _focusreleaseinterpspeed _occlusionlowpassfilterfrequency _occlusionvolumeattenuation _occlusioninterpolationtime _reverbwetlevelmin _reverbwetlevelmax _reverbdistancemin _reverbdistancemax _manualreverbsendlevel _customreverbsendcurve _pluginsettings _distancealgorithm _attenuationshape _dbattenuationatmax _attenuationshapeextents _coneoffset _falloffdistance) (Utilities|Struct|BreakSoundAttenuationSettings _attenuation))
  (bind _x (Math|Vector|BreakVector _attenuationshapeextents))
  (bind _returnvalue (+ _x _falloffdistance))
  (bind _returnvalue_2 (/ _returnvalue 3e+01))
  (Utilities|IsValid _attenuationsettings
    (:Is%20Valid
      (Transformation|SetWorldScale3D (Variables|Default|GetSphere) (Math|Vector|MakeVector _returnvalue_2 _returnvalue_2 _returnvalue_2)))))

(fn PlayWordatPhraseLocation
  (params (InSound :type Sound%20Base%20Object%20Reference))
  ;[1 1 1] Verify Valid Sound Base
  (Utilities|IsValid InSound
    (:Is%20Valid
      ;[1 1 1] Play Sound with Input Values (Including Randomized Range Values)
      (Audio|PlaySoundatLocation InSound (+ (Transformation|GetWorldLocation (Variables|Default|GetDefaultSceneRoot)) (Variables|Default|GetPhraseLocation)) "0, 0, 0" (* (Math|Random|RandomFloatinRange (Variables|VolumeParameters|GetMinVolumeRange) (Variables|VolumeParameters|GetMaxVolumeRange)) (Variables|VolumeParameters|GetVolumeScale)) (* (Math|Random|RandomFloatinRange (Variables|PitchParameters|GetMinPitchRange) (Variables|PitchParameters|GetMaxPitchRange)) (Variables|PitchParameters|GetPitchScale)) 0.0 (Variables|MainParameters|GetAttenuationSettings) (Variables|MainParameters|GetConcurrencySettings) self))))

(fn EndOfPhraseAction
  (return true))