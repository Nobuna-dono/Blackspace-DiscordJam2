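; Audio hint actor that plays a randomized-volume and pitch sound at its location and lights a sphere's material while active, with a pick-up area for the player.
; CallHint plays the sound and enables Tick for Duration, then resets the glow.
; Tick sets a dynamic material's Intensity from the SoundWave's single-bucket amplitude, lerped by DeltaSeconds.
; EnableHints disables auto-start and shows the actor; player overlap with PickArea calls OnPick.
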(event OnComponentBeginOverlap(PickArea)
  (params (OverlappedComponent :type Primitive%20Component%20Object%20Reference) (OtherActor :type Actor%20Object%20Reference) (OtherComp :type Primitive%20Component%20Object%20Reference) (OtherBodyIndex :type Integer) (bFromSweep :type Boolean) (SweepResult :type Hit%20Result%20Structure%20%28by%20ref%29))
  (if (== OtherActor (Game|Player|GetPlayerPawn 0))
    (Default|CallOnPick)))

(event Custom|CallHint
  (CallFunction|PlayHint)
  (Variables|Default|SetActivated true)
  (CallFunction|Timer)
  (Actor|Tick|SetActorTickEnabled true))

(event Custom|Timer
  (Utilities|FlowControl|Delay (Variables|Default|GetDuration))
  (Variables|Default|SetActivated false)
  (Rendering|Material|SetScalarParameterValue (Variables|Default|GetPulsingMat) "Intensity" 0.0 :!class /Script/Engine.MaterialInstanceDynamic)
  (Actor|Tick|SetActorTickEnabled false))

(event Custom|EnableHints
  (Variables|Default|SetAutoStart false)
  (|CallParentFunction)
  (Rendering|SetVisibility (Variables|Default|GetDefaultSceneRoot) true true))

(event EventBeginPlay)

(event Collision|EventActorBeginOverlap
  (params (OtherActor :type Actor%20Object%20Reference)))

(event EventTick
  (params (DeltaSeconds :type Float%20%28single-precision%29))
  (if (Variables|Default|GetActivated)
    (bind _outamplitudes (Class|SoundVisualizationStatics|GetAmplitude (Variables|Default|GetSoundToEmit) 0 0.0 (Variables|Default|GetDuration) 1))
    (bind _output_get (Variables|Default|SetAmplitude _outamplitudes))
    (Rendering|Material|SetScalarParameterValue (Variables|Default|GetPulsingMat) "Intensity" (Math|Float|Lerp (Variables|Default|GetValueToLerp) (Utilities|Array|Get(acopy) _output_get) DeltaSeconds) :!class /Script/Engine.MaterialInstanceDynamic)))

(fn ConstructionScript
  (|CallParentFunction)
  (bind _returnvalue (Rendering|Material|CreateDynamicMaterialInstance (Variables|Default|GetSphere1) 0 (Rendering|Material|GetMaterial (Variables|Default|GetSphere1) 0) "None" :!class /Script/Engine.PrimitiveComponent))
  (bind _output_get (Variables|Default|SetPulsingMat _returnvalue))
  (Rendering|Material|SetScalarParameterValue _output_get "Intensity" 0.0 :!class /Script/Engine.MaterialInstanceDynamic))

(fn PlayHint
  (bind _volumescale (Variables|Default|GetVolumeScale))
  (Audio|PlaySoundatLocation (Variables|Default|GetSoundToEmit) (Transformation|GetWorldLocation (Variables|Default|GetDefaultSceneRoot)) "0, 0, 0" (* (Math|Random|RandomFloatinRange (Variables|Default|GetMinVolume) (Variables|Default|GetMaxVolume)) (select (Utilities|IsValid _volumescale) (Variables|/Game/1-PROJECT_LDJ/Production/Blueprints/Assets/FloatVariable.FloatVariable_C|GetValue _volumescale) 1.0)) (* (Math|Random|RandomFloatinRange (Variables|Default|GetMinPitch) (Variables|Default|GetMaxPitch)) (Variables|Default|GetPitchScale)) 0.0 (Variables|Default|GetAttenuation) (Variables|Default|GetConcurrencySettings) self))